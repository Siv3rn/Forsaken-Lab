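; Interactable password lock that opens or closes a linked door through an on-screen numpad.
; On BeginPlay it creates the WB_Numpad widget, passes it the door password and binds its correct and false events.
; Interact flip-flops the numpad, switching input mode, cursor and movement lock.
; A correct code toggles the door, a wrong one plays an alarm sound, and both call ExitNumpad to close the UI.
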(event `/Game/FirstPerson/Blueprints/BPI_Interactable.Interact`
  (bind _returnvalue (`GameplayStatics.GetPlayerController` 0))
  (bind _numpadui (`self.NumpadUI`))
  (bind _numpad (`/Game/UI/WB_Numpad.Numpad` _numpadui))
  (`|ExecutionSequence`
    (:`then_0`
      (if (`self.IsInteractable`)
        (`/Engine/EditorBlueprintResources/StandardMacros.FlipFlop`
          (:`A`
            (set `Widget.Visibility` "Visible" _numpad)
            (`WidgetBlueprintLibrary.SetInputMode_GameAndUIEx` _returnvalue _numpadui)
            (set `PlayerController.bShowMouseCursor` true _returnvalue)
            (`Controller.SetIgnoreMoveInput` _returnvalue true))
          (:`B`
            (set `Widget.Visibility` "Hidden" _numpad :!label _label)
            (`WidgetBlueprintLibrary.SetInputMode_GameOnly` _returnvalue)
            (set `PlayerController.bShowMouseCursor` false _returnvalue)
            (`Controller.SetIgnoreMoveInput` _returnvalue false)
            (`/Game/UI/WB_Numpad.Clear` (`self.NumpadUI`))))))))

(event `ExitNumpad`
  (goto _label))

(event `self.ReceiveBeginPlay`
  (bind _returnvalue (`|CreateWidget` "/Game/UI/WB_Numpad.WB_Numpad_C"))
  (bind _output_get (set `self.NumpadUI` _returnvalue))
  (`UserWidget.AddToViewport` _output_get 0)
  (set `/Game/UI/WB_Numpad.Correct Password` (`KismetStringLibrary.Conv_IntToString` (`self.DoorPassword`)) _returnvalue)
  (add `/Game/UI/WB_Numpad.OnCorrect` _returnvalue (delegate `OpenDoor`))
  (add `/Game/UI/WB_Numpad.OnFalse` _returnvalue (delegate `Alarm`)))

(event `Alarm`
  (`GameplayStatics.PlaySoundAtLocation` "/Game/SoundFX/SQ_Alarm.SQ_Alarm" (`self.K2_GetActorLocation` self) (struct) 1.0 1.0 0.0 null null null null)
  (`self.ExitNumpad`))

(event `OpenDoor`
  (bind _door (`self.Door`))
  (if (`/Game/Environtment/BP_ElectricDoor.IsClose` _door)
    (`/Game/Environtment/BP_ElectricDoor.OpenDoor` _door)
    (else
      (`/Game/Environtment/BP_ElectricDoor.CloseDoor` _door)))
  (`self.ExitNumpad`))

(fn `GetInteractText`
  (returns (InteractText :type String))
  (return (`self.Interact Text`)))

(fn `UserConstructionScript`)