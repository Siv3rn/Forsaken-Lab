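; Trigger volume that plays a monologue on the player character when the player enters it.
; BeginPlay caches the BP_FirstPersonCharacter reference, and a DoOnce gates the overlap before the player check, so the first overlap by any actor consumes it.
; A delayed loop bounded by Speech's length calls StartMonologue at three-second intervals, passing the whole Speech rather than an indexed line.
; An array of story dialogue sits unconnected in the graph.
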(event `self.ReceiveBeginPlay`
  (bind _asbp_first_person_character (cast `/Game/FirstPerson/Blueprints/BP_FirstPersonCharacter` (`GameplayStatics.GetPlayerCharacter` 0)))
  (set `self.MCRef` _asbp_first_person_character))

(event `self.TriggerZone.OnComponentBeginOverlap`
  (params (OverlappedComponent :type "PrimitiveComponent Object Reference") (OtherActor :type "Actor Object Reference") (OtherComp :type "PrimitiveComponent Object Reference") (OtherBodyIndex :type Integer) (bFromSweep :type Boolean) (SweepResult :type "HitResult Structure (by ref)"))
  (bind _speech (`self.Speech`))
  (`/Engine/EditorBlueprintResources/StandardMacros.DoOnce` false
    (:`Completed`
      (if (== OtherActor (`GameplayStatics.GetPlayerCharacter` 0))
        (`/Game/FirstPerson/Blueprints/BML_ForsakenLab.ForLoopWithDelay` 0 (`KismetArrayLibrary.Array_Length` _speech) 3.0
          (:`LoopBody`
            (`/Game/FirstPerson/Blueprints/BP_FirstPersonCharacter.StartMonologue` (`self.MCRef`) _speech)))))))

(fn `UserConstructionScript`)