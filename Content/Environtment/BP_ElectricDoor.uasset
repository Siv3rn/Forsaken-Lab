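; BP_ElectricDoor is a two-panel sliding door actor with open and close events that play a sliding sound at its location.
; Each event runs a timeline that moves Door2's relative location, whose Update starts a second timeline that moves Door1 and sets the IsClose flag.
; Opening and closing use separate timeline pairs, with closing playing Door2's timeline in reverse and Door1's forward.
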(event `OpenDoor`
  (`GameplayStatics.PlaySoundAtLocation` "/Game/SoundFX/SlidingDoor.SlidingDoor" (`self.K2_GetActorLocation` self) (struct) 1.0 1.0 0.0 null null null null)
  (bind (_direction _door_location) (`Timeline|Timeline` :!via `PlayFromStart`)
    (:`Update`
      (`SceneComponent.K2_SetRelativeLocation` (`self.Door2`) _door_location false false)
      (bind (_direction_2 _door_location_2) (`Timeline|Timeline_1`)
        (:`Update`
          (`SceneComponent.K2_SetRelativeLocation` (`self.Door1`) _door_location_2 false false)
          (set `self.IsClose` false))))))

(event `CloseDoor`
  (`GameplayStatics.PlaySoundAtLocation` "/Game/SoundFX/SlidingDoor.SlidingDoor" (`self.K2_GetActorLocation` self) (struct) 1.0 1.0 0.0 null null null null)
  (bind (_direction _door_location) (`Timeline|Timeline_0` :!via `ReverseFromEnd`)
    (:`Update`
      (`SceneComponent.K2_SetRelativeLocation` (`self.Door2`) _door_location false false)
      (bind (_direction_2 _door_location_2) (`Timeline|Timeline_2`)
        (:`Update`
          (`SceneComponent.K2_SetRelativeLocation` (`self.Door1`) _door_location_2 false false)
          (set `self.IsClose` true))))))

(fn `UserConstructionScript`)