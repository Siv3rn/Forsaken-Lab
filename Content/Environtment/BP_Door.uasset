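; BP_Door is an interactable door that can be locked behind a required item and swings open or shut.
; On Interact, a locked door checks the first-person character's ItemManager for its Requirement, then either unlocks or prints a locked message.
; An unlocked door uses a FlipFlop to play or reverse the OpenDoor timeline, which lerps the Door's yaw through a quarter turn.
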(event `/Game/FirstPerson/Blueprints/BI_Interactable.Interact`
  (if (`self.isLocked`)
    (bind _havekeys (`self.CheckKeys`))
    (if _havekeys
      (set `self.isLocked` false)
      (else
        (`KismetSystemLibrary.PrintString` "It's Locked")))
    (else
      (`/Engine/EditorBlueprintResources/StandardMacros.FlipFlop`
        (:`A`
          (bind (_direction _doorfloat) (`Timeline|OpenDoor` :!via `PlayFromStart` :!label _label)
            (:`Update`
              (`SceneComponent.K2_SetRelativeRotation` (`self.Door`) (`KismetMathLibrary.MakeRotator` 0.0 0.0 (`KismetMathLibrary.Lerp` 0.0 90.0 _doorfloat)) false false))))
        (:`B`
          (goto _label :!via `Reverse`))))))

(fn `CheckKeys`
  (returns (HaveKeys :type Boolean))
  (bind _asbp_first_person_character (cast `/Game/FirstPerson/Blueprints/BP_FirstPersonCharacter` (`GameplayStatics.GetPlayerPawn` 0)))
  (if (`KismetArrayLibrary.Array_Contains` (`/Game/FirstPerson/Blueprints/BP_FirstPersonCharacter.itemManager` _asbp_first_person_character) (`self.Requirement`))
    (return true)
    (else
      (return false))))

(fn `UserConstructionScript`)