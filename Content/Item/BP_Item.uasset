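; BP_Item is an interactable pickup actor that the first-person player character can collect.
; On Interact it passes itself to the character's PickUpItem, sets its State to the picked-up value, then hides and disables collision.
; On BeginPlay it loops over the game instance's saved ItemState array, applying each entry to its visibility and collision without index matching, so the last entry wins.
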(event `self.ReceiveTick`
  (params (DeltaSeconds :type "Float (single-precision)")))

(event `self.ReceiveBeginPlay`
  (bind _savegamedata (message `/Game/GameManager/BPI_SaveGame.GetGameData` (`GameplayStatics.GetGameInstance`)))
  (`/Engine/EditorBlueprintResources/StandardMacros.IsValid` _savegamedata
    (:`Is Valid`
      (for _array_element (`/Game/GameManager/BP_Save.ItemState` _savegamedata)
        (set `self.State` _array_element)
        (if (`|EnumEquality` (`self.State`) "NewEnumerator5")
          (`self.SetActorEnableCollision` false)
          (`self.SetActorHiddenInGame` true)
          (else
            (`self.SetActorEnableCollision` true)
            (`self.SetActorHiddenInGame` false)))))))

(event `/Game/FirstPerson/Blueprints/BI_Interactable.Interact`
  (bind _asbp_first_person_character (cast `/Game/FirstPerson/Blueprints/BP_FirstPersonCharacter` (`GameplayStatics.GetPlayerPawn` 0)))
  (`/Game/FirstPerson/Blueprints/BP_FirstPersonCharacter.PickUpItem` _asbp_first_person_character self)
  (set `self.State` "NewEnumerator5")
  (`self.SetActorEnableCollision` false)
  (`self.SetActorHiddenInGame` true))

(fn `UserConstructionScript`)