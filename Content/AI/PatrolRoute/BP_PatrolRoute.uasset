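; BP_PatrolRoute is an AI patrol route actor that supplies world-space patrol points from a spline.
; IncreamentPatrolRoute sets PatrolIndex to a random spline point index, then offsets it by Direction, so progression is random rather than sequential.
; Direction flips when the result lands exactly on the first or last point, with no clamping.
; GetSplinePointsAsWorldLocation returns the world location of the point at PatrolIndex.
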(event `IncreamentPatrolRoute`
  ;[1 1 1] Increament Patrol Point
  ;;[1 1 1] Set Random Point
  (set `self.PatrolIndex` (`KismetMathLibrary.RandomInteger` (- (`SplineComponent.GetNumberOfSplinePoints` (`self.PatrolRoute`)) 1)))
  (bind _output_get (set `self.PatrolIndex` (+ (`self.PatrolIndex`) (`self.Direction`))))
  (if (== _output_get (- (`SplineComponent.GetNumberOfSplinePoints` (`self.PatrolRoute`)) 1))
    (set `self.Direction` -1)
    (elif (== (`self.PatrolIndex`) 0)
      (set `self.Direction` 1))))

(fn `GetSplinePointsAsWorldLocation`
  (returns (ReturnValue :type "Vector Structure"))
  (return (`SplineComponent.GetLocationAtSplinePoint` (`self.PatrolRoute`) (`self.PatrolIndex`) "World")))

(fn `UserConstructionScript`)