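; Enemy AI character that hunts the player by sight and kills them with a jumpscare on contact.
; Sight perception updates set or clear the blackboard TargetActor and store LastKnownLocation when the player is lost.
; Player overlap with JumpscareCollision applies a single interpolated rotation step, then after a short delay plays the attack montage and jumpscare sound and calls DIE on the cached player character.
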(event `self.ReceiveBeginPlay`
  (bind _asbp_first_person_character (cast `/Game/FirstPerson/Blueprints/BP_FirstPersonCharacter` (`GameplayStatics.GetPlayerCharacter` 0)))
  (set `self.MCRef` _asbp_first_person_character))

(event `self.ReceiveTick`
  (params (DeltaSeconds :type "Float (single-precision)")))

(event `self.AIPerception.OnTargetPerceptionUpdated`
  (params (Actor :type "Actor Object Reference") (Stimulus :type "AIStimulus Structure"))
  (`self.HandleSightSense` Actor Stimulus))

(event `self.JumpscareCollision.OnComponentBeginOverlap`
  (params (OverlappedComponent :type "PrimitiveComponent Object Reference") (OtherActor :type "Actor Object Reference") (OtherComp :type "PrimitiveComponent Object Reference") (OtherBodyIndex :type Integer) (bFromSweep :type Boolean) (SweepResult :type "HitResult Structure (by ref)"))
  (bind _returnvalue (`GameplayStatics.GetPlayerCharacter` 0))
  (if (== OtherActor _returnvalue)
    (`self.K2_SetActorRotation` (`KismetMathLibrary.RInterpTo` (`KismetMathLibrary.FindLookAtRotation` (`self.K2_GetActorLocation`) (`self.K2_GetActorLocation` _returnvalue)) (`self.GetControlRotation`) (`GameplayStatics.GetWorldDeltaSeconds`) 2.0))
    (`KismetSystemLibrary.Delay` 0.2)
    (`self.PlayAnimMontage` "/Game/Animation/AM_EnemyAttack.AM_EnemyAttack")
    (`GameplayStatics.PlaySound2D` "/Game/SoundFX/SQ_Jumpscare.SQ_Jumpscare" 1.0 1.0 0.0 null null)
    (`/Game/FirstPerson/Blueprints/BP_FirstPersonCharacter.DIE` (`self.MCRef`) self)))

(fn `HandleSightSense`
  (params (Actor :type "Actor Object Reference") (Stimulus :type "AIStimulus Structure"))
  (bind (_stimulus_age _stimulus_expirationage _stimulus_strength _stimulus_stimuluslocation _stimulus_receiverlocation _stimulus_tag _stimulus_bsuccessfullysensed) (break `AIStimulus` (`local.Stimulus`)))
  (bind _returnvalue (`AIBlueprintHelperLibrary.GetBlackboard` (`AIBlueprintHelperLibrary.GetAIController` self)))
  (bind _returnvalue_2 (`AIPerceptionSystem.GetSenseClassForStimulus` Stimulus))
  (if (== _returnvalue_2 "/Script/AIModule.AISense_Sight")
    (if (== (`GameplayStatics.GetPlayerCharacter` 0) (`local.Actor`))
      (`BlackboardComponent.SetValueAsObject` _returnvalue "TargetActor" (`KismetMathLibrary.SelectObject` (`GameplayStatics.GetPlayerCharacter` 0) null _stimulus_bsuccessfullysensed))
      (if (not _stimulus_bsuccessfullysensed)
        (`BlackboardComponent.SetValueAsVector` _returnvalue "LastKnownLocation" _stimulus_stimuluslocation))
      (else
        (return)))
    (else
      (return))))

(fn `UserConstructionScript`)